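; Base gun Blueprint that handles firing, ammo and reloading for a player passed into FireGun.
; FireGun branches on fire type to single, auto, burst (a delayed loop with no exit) or shotgun logic.
; Shots trace from the active camera (shotgun: FPP only, randomized pellets), then spawn bullets from the muzzle arrow toward the hit via the player's ROSSpawnActor.
; Empty clips trigger montage-timed reloads from reserve ammo.
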(event Custom|Fire%20Gun
  (params (Firing :type Boolean) (Player%20Ref :type Player%20Character%20BP%20Object%20Reference))
  ;[1 1 1] Fire Gun
  (Variables|Default|SetPlayer%20Ref Player%20Ref)
  (bind _output_get (Variables|Default|SetFiring Firing))
  (if _output_get
    (switch Utilities|FlowControl|Switch|SwitchonFireTypes (Variables|GunSettings|GetFireType)
      (:NewEnumerator0
        (CallFunction|Shoot))
      (:NewEnumerator1
        (CallFunction|FireBurst))
      (:NewEnumerator2
        (CallFunction|FireAuto))
      (:NewEnumerator3
        (CallFunction|ShotgunShoot)))))

(event Custom|Shotgun%20Shoot
  (bind _player_ref (Variables|Default|GetPlayer%20Ref))
  (bind _arrow (Variables|Default|GetArrow))
  (bind _player_ref_2 (Variables|Default|GetPlayer%20Ref))
  (bind _returnvalue (Transformation|GetWorldLocation _arrow))
  (bind _fpp_cam (Variables|/Game/Blueprints/PlayerBlueprint/PlayerCharacterBP.PlayerCharacterBP_C|GetFPP%20Cam _player_ref))
  (bind _returnvalue_2 (Transformation|GetWorldLocation _fpp_cam))
  ;[1 1 1] Fire Shotgun
  (Utilities|FlowControl|Sequence
    (:then_0
      (if (not (Variables|Default|GetShooting))
        (if (> (Variables|Ammo|GetAmmo) 0)
          (Math|Integer|DecrementInt (Variables|Ammo|GetAmmo)
            (:%20%20
              (Default|PlayMontage (Variables|Default|GetPlayer%20Ref) (Variables|GunSettings|GetFire%20Anim) 1.0 "None")
              (Components|Animation|PlayAnimation (Variables|Default|GetSkeletalMesh) (Variables|GunSettings|GetFire%20Anim_Gun) false)
              (for _index (range 1 (Math|Random|RandomIntegerinRange 6 9))
                (bind (_outhit _returnvalue_3) (Collision|LineTraceByChannel _returnvalue_2 (+ (+ _returnvalue_2 (* (Math|Vector|GetForwardVector _fpp_cam) 5e+03)) (Math|Vector|MakeVector (Math|Random|RandomFloatinRange -1e+02 1e+02) (Math|Random|RandomFloatinRange -1e+02 1e+02) (Math|Random|RandomFloatinRange -1e+02 1e+02))) "TraceTypeQuery1" true 0 "None"))
                (Default|ROSSpawnActor _player_ref_2 (Variables|GunSettings|GetBullet) (Math|Transform|MakeTransform _returnvalue (Math|Rotator|FindLookatRotation _returnvalue (Math|Vector|SelectVector (.ImpactPoint (Collision|BreakHitResult _outhit)) (.TraceEnd (Collision|BreakHitResult _outhit)) _returnvalue_3))) "AlwaysSpawn" _player_ref_2))))
          (else
            (CallFunction|Reload)))))
    (:then_1
      (Utilities|FlowControl|Delay (Variables|GunSettings|GetDelay%20Between%20Shots))
      (Variables|Default|SetShooting false))))

(event Custom|Fire%20Auto
  ;[1 1 1] Single And Burst Shots
  (if (Variables|Default|GetFiring) :!label _label
    (CallFunction|Shoot)
    (Utilities|FlowControl|Delay (Variables|GunSettings|GetDelay%20Between%20Shots))
    (goto _label)))

(event Custom|Fire%20Burst
  ;[1 1 1] Single And Burst Shots
  (Utilities|FlowControl|Sequence
    (:then_0
      _)
    (:then_1
      (Utilities|FlowControl|Delay (Variables|GunSettings|GetDelay%20Between%20Shots))))
  (CallFunction|Shoot))

(event Custom|Reload
  (bind _player_ref (Variables|Default|GetPlayer%20Ref))
  ;[1 1 1] Reload
  (if (not (Variables|Default|GetRelaoding))
    (Variables|Default|SetRelaoding true)
    (if (> (Variables|Ammo|GetMax%20Ammo) 0)
      (Variables|Default|SetFiring false)
      (Default|ADSCam _player_ref false)
      (bind _anim_duration (Default|PlayMontage _player_ref (Variables|GunSettings|GetReload%20Anim) 1.0 "None"))
      (Components|Animation|PlayAnimation (Variables|Default|GetSkeletalMesh) (Variables|GunSettings|GetReload%20Anim_Gun) false)
      (Utilities|FlowControl|Delay _anim_duration)
      (Variables|Default|SetRelaoding false)
      ;;[0.135 0 1] Reaload Code
      (if (> (Variables|Ammo|GetMax%20Ammo) (Variables|Ammo|GetAmmo%20Clip%20Size))
        (Variables|Ammo|SetMax%20Ammo (- (Variables|Ammo|GetMax%20Ammo) (- (Variables|Ammo|GetAmmo%20Clip%20Size) (Variables|Ammo|GetAmmo))))
        (Variables|Ammo|SetAmmo (Variables|Ammo|GetAmmo%20Clip%20Size))
        (else
          (Variables|Ammo|SetAmmo (Variables|Ammo|GetMax%20Ammo))
          (Variables|Ammo|SetMax%20Ammo 0)))
      (else
        (Variables|Default|SetRelaoding false)))))

(event Custom|Shoot
  (bind _player_ref (Variables|Default|GetPlayer%20Ref))
  (bind _arrow (Variables|Default|GetArrow))
  (bind _player_ref_2 (Variables|Default|GetPlayer%20Ref))
  (bind _ads_cam (Variables|Default|GetADS%20Cam))
  (bind _returnvalue (Transformation|GetWorldLocation _arrow))
  (bind _ads (Variables|/Game/Blueprints/PlayerBlueprint/PlayerCharacterBP.PlayerCharacterBP_C|GetADS _player_ref))
  (bind _fpp_cam (Variables|/Game/Blueprints/PlayerBlueprint/PlayerCharacterBP.PlayerCharacterBP_C|GetFPP%20Cam _player_ref))
  (bind _returnvalue_2 (select _ads _ads_cam _fpp_cam))
  (bind _returnvalue_3 (Transformation|GetWorldLocation _returnvalue_2))
  ;[1 1 1] Shoot
  (Utilities|FlowControl|Sequence
    (:then_0
      (if (not (Variables|Default|GetShooting))
        (Variables|Default|SetShooting true)
        (if (not (Variables|Default|GetRelaoding))
          (if (> (Variables|Ammo|GetAmmo) 0)
            (Math|Integer|DecrementInt (Variables|Ammo|GetAmmo)
              (:%20%20
                (Default|PlayMontage (Variables|Default|GetPlayer%20Ref) (Variables|GunSettings|GetFire%20Anim) 1.0 "None")
                (Components|Animation|PlayAnimation (Variables|Default|GetSkeletalMesh) (Variables|GunSettings|GetFire%20Anim_Gun) false)
                (bind (_outhit _returnvalue_4) (Collision|LineTraceByChannel _returnvalue_3 (+ _returnvalue_3 (* (Math|Vector|GetForwardVector _returnvalue_2) 9999.0)) "TraceTypeQuery1" true 0 "None"))
                (Default|ROSSpawnActor _player_ref_2 (Variables|GunSettings|GetBullet) (Math|Transform|MakeTransform _returnvalue (Math|Rotator|FindLookatRotation _returnvalue (Math|Vector|SelectVector (.ImpactPoint (Collision|BreakHitResult _outhit)) (.TraceEnd (Collision|BreakHitResult _outhit)) _returnvalue_4))) "AlwaysSpawn" _player_ref_2)))
            (else
              (CallFunction|Reload))))))
    (:then_1
      (Utilities|FlowControl|Delay (Variables|GunSettings|GetDelay%20Between%20Shots))
      (Variables|Default|SetShooting false))))

(event EventBeginPlay)

(event Collision|EventActorBeginOverlap
  (params (OtherActor :type Actor%20Object%20Reference)))

(event EventTick
  (params (DeltaSeconds :type Float%20%28single-precision%29)))

(fn ConstructionScript)