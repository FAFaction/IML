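; Gun spawner actor that places a weapon through a child actor component named Gun.
; The construction script sets the child actor class from the Guns variable.
; On Tick, a 10-second Delay gates a check that sets the class again when the child actor is no longer valid, respawning the gun.
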(event EventBeginPlay)

(event Collision|EventActorBeginOverlap
  (params (OtherActor :type Actor%20Object%20Reference)))

(event EventTick
  (params (DeltaSeconds :type Float%20%28single-precision%29))
  (Utilities|FlowControl|Delay 1e+01)
  (Utilities|IsValid (Variables|/Script/Engine.ChildActorComponent|GetChildActor (Variables|Default|GetGun))
    (:Is%20Not%20Valid
      (ChildActorComponent|SetChildActorClass (Variables|Default|GetGun) (Variables|Default|GetGuns)))))

(fn ConstructionScript
  (ChildActorComponent|SetChildActorClass (Variables|Default|GetGun) (Variables|Default|GetGuns)))