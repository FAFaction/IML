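; Arena actor that runs a two-player deathmatch, tracking each player's score.
; A Tick-plus-Delay countdown triggers a one-time start that creates the arena UI, finds both player characters and moves them to PlayerStarts.
; Each player's no-health event awards the opponent a point, then returns the victim to their start and calls ROSHealth.
; Score updates pass an authority check into MC events; win-score checks have no outcome yet.
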(event Custom|Set%20Up%20Player
  (Utilities|FlowControl|Sequence
    (:then_0
      (bind _outactors (Actor|GetAllActorsOfClass "/Game/Blueprints/PlayerBlueprint/PlayerCharacterBP.PlayerCharacterBP_C"))
      (Utilities|IsValid (Utilities|Array|Get(acopy) _outactors)
        (:Is%20Valid
          (bind _output_get (Variables|Default|SetPlayer1 (Utilities|Array|Get(acopy) _outactors)))
          (Variables|Default|SetPlayer%201%20controller (Pawn|GetController _output_get))
          (EventDispatchers|BindEventtoOnNoHealth (Variables|/Game/Blueprints/PlayerBlueprint/PlayerCharacterBP.PlayerCharacterBP_C|GetHealth_Damage_Component (Variables|Default|GetPlayer1)) (delegate Custom|BlueKills)))))
    (:then_1
      (bind _outactors_2 (Actor|GetAllActorsOfClass "/Game/Blueprints/PlayerBlueprint/PlayerCharacterBP.PlayerCharacterBP_C"))
      (Utilities|IsValid (Utilities|Array|Get(acopy) _outactors_2 1)
        (:Is%20Valid
          (bind _output_get_2 (Variables|Default|SetPlayer2 (Utilities|Array|Get(acopy) _outactors_2 1)))
          (Variables|Default|SetPlayer%202%20Controller (Pawn|GetController _output_get_2))
          (EventDispatchers|BindEventtoOnNoHealth (Variables|/Game/Blueprints/PlayerBlueprint/PlayerCharacterBP.PlayerCharacterBP_C|GetHealth_Damage_Component (Variables|Default|GetPlayer2)) (delegate Custom|RedKills)))))))

(event Custom|RedKills
  (bind _player2 (Variables|Default|GetPlayer2))
  (CallFunction|SetPlayer1Score (+ (Variables|Default|GetPlayer%201%20Score) 1))
  (Utilities|FlowControl|Sequence
    (:then_0
      (if (== (Variables|Default|GetPlayer%201%20Score) (Variables|Default|GetWin%20Score))
        _))
    (:then_1
      (bind _outactors (Actor|GetAllActorsOfClass "/Script/Engine.PlayerStart"))
      (Transformation|SetActorLocation _player2 (.location (Transformation|GetActorTransform (Utilities|Array|Get(acopy) _outactors 1))) false false)
      (Default|ROSHealth (Variables|/Game/Blueprints/PlayerBlueprint/PlayerCharacterBP.PlayerCharacterBP_C|GetHealth_Damage_Component _player2) 1e+02))))

(event Custom|MC%20Player%202%20Score
  (params (Player%202%20Score :type Integer))
  (bind _output_get (Variables|Default|SetPlayer%202%20Score Player%202%20Score))
  (Development|PrintString (Utilities|String|ToString(Integer) _output_get)))

(event Custom|MC%20Player1%20Score
  (params (Player%201%20Score :type Integer))
  (bind _output_get (Variables|Default|SetPlayer%201%20Score Player%201%20Score))
  (Development|PrintString (Utilities|String|ToString(Integer) _output_get)))

(event Custom|Set%20Player%201%20Score
  (params (Player%201%20Score :type Integer))
  (Networking|SwitchHasAuthority
    (:Authority
      (CallFunction|MCPlayer1Score Player%201%20Score))))

(event Custom|Set%20Player%202%20Score
  (params (Player%202%20Score :type Integer))
  (Networking|SwitchHasAuthority
    (:Authority
      (CallFunction|MCPlayer2Score Player%202%20Score))))

(event Custom|BlueKills
  (bind _player1 (Variables|Default|GetPlayer1))
  (CallFunction|SetPlayer2Score (+ (Variables|Default|GetPlayer%202%20Score) 1))
  (Utilities|FlowControl|Sequence
    (:then_0
      (bind _outactors (Actor|GetAllActorsOfClass "/Script/Engine.PlayerStart"))
      (Transformation|SetActorLocation _player1 (.Location (Math|Transform|BreakTransform (Transformation|GetActorTransform (Utilities|Array|Get(acopy) _outactors)))) false false)
      (Default|ROSHealth (Variables|/Game/Blueprints/PlayerBlueprint/PlayerCharacterBP.PlayerCharacterBP_C|GetHealth_Damage_Component _player1) 1e+02))
    (:then_1
      (if (== (Variables|Default|GetPlayer%202%20Score) (Variables|Default|GetWin%20Score))
        _))))

(event EventBeginPlay)

(event EventTick
  (params (DeltaSeconds :type Float%20%28single-precision%29))
  (bind _player2 (Variables|Default|GetPlayer2))
  (Utilities|FlowControl|Delay 1.0)
  (bind _output_get (Variables|Default|SetGame%20Start%20Time (- (Variables|Default|GetGame%20Start%20Time) 1)))
  (if (== _output_get 0)
    (Utilities|FlowControl|DoOnce false
      (:Completed
        (bind _returnvalue (UserInterface|CreateWidget "/Game/Blueprints/CustomBlueprints/ArenaUI.ArenaUI_C" 0 self))
        (UserInterface|Viewport|AddtoPlayerScreen _returnvalue)
        (CallFunction|SetUpPlayer)
        (bind _outactors (Actor|GetAllActorsOfClass "/Script/Engine.PlayerStart"))
        (Transformation|SetActorLocation (Variables|Default|GetPlayer1) (Transformation|GetActorLocation (Utilities|Array|Get(acopy) _outactors)) false false)
        (bind _outactors_2 (Actor|GetAllActorsOfClass "/Script/Engine.PlayerStart"))
        (Utilities|IsValid _player2
          (:Is%20Valid
            (Transformation|SetActorLocation _player2 (Transformation|GetActorLocation (Utilities|Array|Get(acopy) _outactors_2 1)) false false)))))))

(fn ConstructionScript)