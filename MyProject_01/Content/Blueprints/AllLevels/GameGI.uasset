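; GameGI is a Game Instance that handles online session hosting, searching and joining, and auto-configures graphics settings on Init.
; Init runs a hardware benchmark and applies the results to Game User Settings.
; CreateGame creates a non-LAN session, then opens GameTestMap as a listen server.
; FindGame refills SessionsFound and calls FindingSessionComplete, or NoSessionsFound when the search fails, while JoinGame joins the passed session.
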(event Custom|Create%20Game
  ;[1 1 1] Find And Join Games
  (|Session (Game|GetPlayerController 0) 100 false
    (:OnSuccess
      (Game|OpenLevel(byName) "GameTestMap" true "listen"))))

(event Custom|Find%20Game
  ;[1 1 1] Find And Join Games
  (Utilities|Array|Clear (Variables|Default|GetSessions%20Found))
  (bind _results (|FindSessions (Game|GetPlayerController 0) 100 false)
    (:OnSuccess
      (for _array_element _results
        (Utilities|Array|Add (Variables|Default|GetSessions%20Found) _array_element))
      (Default|CallFindingSessionComplete))
    (:OnFailure
      (Default|CallNoSessionsFound))))

(event Custom|Join%20Game
  (params (Session :type Blueprint%20Session%20Result%20Structure%20%28by%20ref%29))
  ;[1 1 1] Find And Join Games
  (|JoinSession (Game|GetPlayerController 0) Session))

(event EventInit
  (bind _returnvalue (Settings|GetGameUserSettings))
  (Class|GameUserSettings|RunHardwareBenchmark _returnvalue 10 1.0 1.0)
  (Class|GameUserSettings|ApplyHardwareBenchmarkResults _returnvalue))