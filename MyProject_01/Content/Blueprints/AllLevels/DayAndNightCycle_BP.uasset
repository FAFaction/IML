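; Day and night cycle actor that rotates the level's sun and adjusts lighting to match.
; On BeginPlay it caches the first DirectionalLight, SkyLight and BP_Sky_Sphere.
; Each Tick pitches the sun by DayTime-scaled delta time with slight yaw, then updates the sky sphere.
; Sun pitch selects night or day lighting, interpolating skylight intensity and setting sun indirect intensity from its interpolated main intensity.
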(event EventBeginPlay
  (bind _outactors (Actor|GetAllActorsOfClass "/Script/Engine.DirectionalLight"))
  (Variables|Default|SetDirectional%20Light (Utilities|Array|Get(acopy) _outactors))
  (bind _outactors_2 (Actor|GetAllActorsOfClass "/Script/Engine.SkyLight"))
  (Variables|Default|SetSky%20Light (Utilities|Array|Get(acopy) _outactors_2))
  (bind _outactors_3 (Actor|GetAllActorsOfClass "/Engine/EngineSky/BP_Sky_Sphere.BP_Sky_Sphere_C"))
  (Variables|Default|SetSky%20Sphere (Utilities|Array|Get(acopy) _outactors_3)))

(event Collision|EventActorBeginOverlap
  (params (OtherActor :type Actor%20Object%20Reference)))

(event EventTick
  (params (DeltaSeconds :type Float%20%28single-precision%29))
  (bind _day_time (Variables|Default|GetDay%20Time))
  (bind _directional_light (Variables|Default|GetDirectional%20Light))
  (bind _returnvalue (* DeltaSeconds _day_time))
  (Transformation|AddActorLocalRotation _directional_light (Math|Rotator|MakeRotator 0.0 _returnvalue 0.004) false false)
  (Default|UpdateSunDirection (Variables|Default|GetSky%20Sphere))
  (bind _output_get (Variables|Default|SetNight%20Time (Math|Float|InRange(Float) (.pitch (Transformation|GetActorRotation _directional_light)) 0.0 1e+02)))
  (if _output_get
    (CallFunction|NightLighing _returnvalue)
    (else
      (CallFunction|DayLighing _returnvalue))))

(fn ConstructionScript)

(fn NightLighing
  (params (Delta :type Float%20%28single-precision%29))
  (bind _returnvalue (/ Delta 64.0))
  (bind _directional_light (Variables|Default|GetDirectional%20Light))
  (bind _sky_light (Variables|Default|GetSky%20Light))
  (bind _lightcomponent (Variables|/Script/Engine.Light|GetLightComponent _directional_light))
  (bind _lightcomponent_2 (Variables|/Script/Engine.SkyLight|GetLightComponent _sky_light))
  (Class|LightComponent|SetIndirectLightingIntensity _lightcomponent (Math|Interpolation|FInterpTo (Variables|/Script/Engine.LightComponentBase|GetIntensity _lightcomponent) 0.1 _returnvalue 3.0))
  (Rendering|Components|Light|SetIntensity _lightcomponent_2 (Math|Interpolation|FInterpTo (Variables|/Script/Engine.LightComponentBase|GetIntensity _lightcomponent_2) 0.01 _returnvalue 5.0)))

(fn DayLighing
  (params (Delta :type Float%20%28single-precision%29))
  (bind _returnvalue (/ Delta 64.0))
  (bind _directional_light (Variables|Default|GetDirectional%20Light))
  (bind _sky_light (Variables|Default|GetSky%20Light))
  (bind _lightcomponent (Variables|/Script/Engine.Light|GetLightComponent _directional_light))
  (bind _lightcomponent_2 (Variables|/Script/Engine.SkyLight|GetLightComponent _sky_light))
  (Class|LightComponent|SetIndirectLightingIntensity _lightcomponent (Math|Interpolation|FInterpTo (Variables|/Script/Engine.LightComponentBase|GetIntensity _lightcomponent) 3.0 _returnvalue 4.0))
  (Rendering|Components|Light|SetIntensity _lightcomponent_2 (Math|Interpolation|FInterpTo (Variables|/Script/Engine.LightComponentBase|GetIntensity _lightcomponent_2) 0.5 _returnvalue 8.0)))