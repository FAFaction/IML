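; Health component that tracks damage taken by its owning Pawn and signals when health runs out.
; On BeginPlay it binds to the Pawn's OnTakeAnyDamage, then subtracts each hit from Health and prints the result.
; When Health is no longer above zero, it calls the OnNoHealth dispatcher.
; A ROS_Health setter event exists, but its call in the damage logic is disconnected.
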(event Custom|Event%20Any%20Damage%20On%20Pawn
  (params (DamagedActor :type Actor%20Object%20Reference) (Damage :type Float%20%28single-precision%29) (DamageType :type Damage%20Type%20Object%20Reference) (InstigatedBy :type Controller%20Object%20Reference) (DamageCauser :type Actor%20Object%20Reference))
  (bind _output_get (Variables|Default|SetHealth (- (Variables|Default|GetHealth) Damage)))
  (Development|PrintString (Utilities|String|ToString(Float) _output_get))
  (if (not (> (Variables|Default|GetHealth) 0.0))
    (Default|CallOnNoHealth)))

(event Custom|ROS_Health
  (params (Health :type Float%20%28single-precision%29))
  (Variables|Default|SetHealth Health))

(event EventBeginPlay
  (bind _aspawn (Utilities|Casting|CastToPawn (Components|GetOwner)))
  (EventDispatchers|BindEventtoOnTakeAnyDamage _aspawn (delegate Custom|Event%20Any%20Damage%20On%20Pawn)))

(event EventTick
  (params (DeltaSeconds :type Float%20%28single-precision%29)))