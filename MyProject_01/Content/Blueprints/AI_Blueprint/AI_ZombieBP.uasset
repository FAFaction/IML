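; Zombie AI character that wanders the navmesh, chases and melee-attacks visible players, and shies away from direct sunlight.
; Each tick it picks the nearest sensed player with line of sight, and capsule-traces toward the directional light; sun exposure halts new chase orders.
; Traces trigger launches off ledges and onto obstacles, while damage can retarget it onto the attacker.
; Montage, rotation and movement-mode changes route through authority-checked events; LookForShade is never called.
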(event OnComponentBeginOverlap(Sphere)
  (params (OverlappedComponent :type Primitive%20Component%20Object%20Reference) (OtherActor :type Actor%20Object%20Reference) (OtherComp :type Primitive%20Component%20Object%20Reference) (OtherBodyIndex :type Integer) (bFromSweep :type Boolean) (SweepResult :type Hit%20Result%20Structure%20%28by%20ref%29))
  ;[1 1 1] Storing Players
  (bind _asplayer_character_bp (Utilities|Casting|CastToPlayerCharacterBP OtherActor))
  (Utilities|Array|Add (Variables|Default|GetPlayers) _asplayer_character_bp))

(event OnComponentEndOverlap(Sphere)
  (params (OverlappedComponent :type Primitive%20Component%20Object%20Reference) (OtherActor :type Actor%20Object%20Reference) (OtherComp :type Primitive%20Component%20Object%20Reference) (OtherBodyIndex :type Integer))
  ;[1 1 1] Storing Players
  (bind _asplayer_character_bp (Utilities|Casting|CastToPlayerCharacterBP OtherActor))
  (Utilities|Array|RemoveItem (Variables|Default|GetPlayers) _asplayer_character_bp))

(event Custom|Go%20to%20Player
  ;[1 1 1] MOving to player location and attacking
  (Utilities|FlowControl|DoOnce false :!label _label
    (:Completed
      (AI|AIMoveTo self "0, 0, 0" (Variables|Default|GetPlayer%20in%20front) (select (Math|Random|RandomBool) 1.5e+02 8e+01) false
        (:OnSuccess
          (goto _label Reset))
        (:OnFail
          (goto _label Reset))))))

(event Custom|Move
  ;[1 1 1] Move to Random location
  (AI|AIMoveTo self (.RandomLocation (Class|NavigationSystem|GetRandomPointinNavigableRadius (Transformation|GetActorLocation) 5e+03)) 0 5.0 false
    (:OnSuccess
      (Utilities|FlowControl|Delay 5.0)
      (CallFunction|Move))))

(event EventTick
  (params (DeltaSeconds :type Float%20%28single-precision%29))
  ;[1 1 1] Ticking
  (Utilities|FlowControl|Sequence
    (:then_0
      (CallFunction|LookforPlayer)
      (CallFunction|InDirectSunLight)
      (Utilities|JumpDownwhenClosetoEdge)
      (Utilities|JumpUponThings)
      (Utilities|AttackPlayer))
    (:then_1
      (Utilities|FlowControl|Sequence
        (:then_0
          (if (Variables|Default|GetIn%20sun)
            (Utilities|FlowControl|DoOnce false :!label _label
              (:Completed
                (CallFunction|ROSMontage "/Game/GameContent/Animations/WareWolfAnimations/A_avoid_back_Montage.A_avoid_back_Montage")))
            (else
              (goto _label Reset))))
        (:then_1
          (if (Variables|Default|GetIn%20sun)
            (Utilities|FlowControl|Sequence
              (:then_0
                (Utilities|IsValid (Variables|Default|GetPlayer%20in%20front)
                  (:Is%20Valid
                    (CallFunction|ROSSetRotation (Math|Rotator|MakeRotator 0.0 0.0 (.yaw (Math|Rotator|FindLookatRotation (Transformation|GetActorLocation) (Transformation|GetActorLocation (Variables|Default|GetPlayer%20in%20front)))))))))
              (:then_1
                (goto _label Reset)))
            (else
              (Utilities|IsValid (Variables|Default|GetPlayer%20in%20front)
                (:Is%20Valid
                  (CallFunction|GotoPlayer)
                  (goto _label_2 Reset))
                (:Is%20Not%20Valid
                  (Utilities|FlowControl|DoOnce false :!label _label_2
                    (:Completed
                      (Utilities|FlowControl|Delay 5.0)
                      (CallFunction|Move))))))))))))

(event Game|Damage|EventAnyDamage
  (params (Damage :type Float%20%28single-precision%29) (DamageType :type Damage%20Type%20Object%20Reference) (InstigatedBy :type Controller%20Object%20Reference) (DamageCauser :type Actor%20Object%20Reference))
  ;[1 1 1] Getting hit
  (Variables|Default|SetHealth (- Damage (Variables|Default|GetHealth)))
  (CallFunction|ROSMontage "/Game/GameContent/Animations/WareWolfAnimations/A_hit_body_front_Montage.A_hit_body_front_Montage")
  (bind _ascharacter (Utilities|WhenHitMovetoPlayer (Transformation|GetActorLocation DamageCauser))
    (:true
      (bind _asplayer_character_bp (Utilities|Casting|CastToPlayerCharacterBP _ascharacter))
      (Variables|Default|SetPlayer%20in%20front _asplayer_character_bp)
      (CallFunction|GotoPlayer))))

(event Custom|ROS_Montage
  (params (AnimMontage :type Anim%20Montage%20Object%20Reference))
  (Networking|SwitchHasAuthority
    (:Authority
      (Animation|PlayAnimMontage AnimMontage 1.0 "None"))))

(event Custom|ROS_Movement%20mode
  (params (NewMovementMode :type EMovementMode%20Enum :default "MOVE_None"))
  (Networking|SwitchHasAuthority
    (:Authority
      (Pawn|Components|CharacterMovement|SetMovementMode (Variables|Character|GetCharacterMovement) NewMovementMode 0))))

(event Custom|ROS_Set%20Rotation
  (params (NewRotation :type Rotator))
  (Networking|SwitchHasAuthority
    (:Authority
      (Transformation|SetActorRotation NewRotation))))

(fn ConstructionScript)

(fn GEtClosesPlayer
  (params (OtherActor :type Array%20of%20Player%20Character%20BP%20Object%20References))
  (bind _distance_to_all_players (LocalVariables|GetDistance%20to%20all%20players))
  (bind _indexofminvalue (Math|Float|MinOfFloatArray _distance_to_all_players))
  (bind _output (Utilities|Array|Get(acopy) OtherActor _indexofminvalue))
  (for _array_element OtherActor
    (if (Collision|IsOverlappingActor (Variables|Default|GetBox) _array_element :!class /Script/Engine.PrimitiveComponent)
      (Utilities|Array|Add (LocalVariables|GetDistance%20to%20all%20players) (Transformation|GetDistanceTo _array_element))))
  (Utilities|IsValid _output
    (:Is%20Valid
      (return _output))))

(fn LookforPlayer
  (bind _players (Variables|Default|GetPlayers))
  (Utilities|IsValid (Utilities|Array|Get(acopy) _players)
    (:Is%20Valid
      (bind _closes_player (CallFunction|GEtClosesPlayer _players))
      (Utilities|IsValid _closes_player
        (:Is%20Valid
          (bind _outhit (Collision|LineTraceByChannel (+ (Transformation|GetActorLocation) "0, 0,40.000000") (+ (Transformation|GetActorLocation _closes_player) "0, 0,60.000000") "TraceTypeQuery2" true 0 "None"))
          (bind _asplayer_character_bp (Utilities|Casting|CastToPlayerCharacterBP (.HitActor (Collision|BreakHitResult _outhit)))
            (:then
              (Variables|Default|SetPlayer%20in%20front _asplayer_character_bp))
            (:CastFailed
              (Variables|Default|SetPlayer%20in%20front 0))))
        (:Is%20Not%20Valid
          (Variables|Default|SetPlayer%20in%20front 0))))))

(fn InDirectSunLight
  (bind _returnvalue (Transformation|GetActorLocation))
  (bind _outactors (Actor|GetAllActorsOfClass "/Script/Engine.DirectionalLight"))
  (bind (_outhit _returnvalue_2) (Collision|CapsuleTraceByChannel _returnvalue (+ _returnvalue (* (Math|Vector|GetForwardVector (Transformation|GetActorRotation (Utilities|Array|Get(acopy) _outactors))) -99999.0)) 34.0 88.0 "TraceTypeQuery2" false 0 "None" true "(R=0.000000,G=0.233631,B=1.000000,A=1.000000)" "(R=1.000000,G=1.000000,B=1.000000,A=1.000000)"))
  (if _returnvalue_2
    (Variables|Default|SetIn%20sun false)
    (else
      (Variables|Default|SetIn%20sun true))))

(fn LookforShade
  (bind _returnvalue (Transformation|GetActorLocation))
  (if (Variables|Default|GetIn%20sun)
    (bind (_outhit _returnvalue_2) (Class|KismetSystemLibrary|BoxTraceSingleforObjects _returnvalue (+ _returnvalue "0, 0,100.000000") "1000.000000,1000.000000,70.000000" (Transformation|GetActorRotation) (Utilities|Array|MakeArray "ObjectTypeQuery1") false 0 "ForDuration" true :!label _label))
    (if _returnvalue_2
      (LocalVariables|SetNew%20Shade%20Location (.ImpactPoint (Collision|BreakHitResult _outhit)))
      (bind _outactors (Actor|GetAllActorsOfClass "/Script/Engine.DirectionalLight"))
      (bind _returnvalue_3 (Collision|LineTraceForObjects (LocalVariables|GetNew%20Shade%20Location) (+ (LocalVariables|GetNew%20Shade%20Location) (* (Math|Vector|GetForwardVector (Transformation|GetActorRotation (Utilities|Array|Get(acopy) _outactors))) -99999.0)) (Utilities|Array|MakeArray "ObjectTypeQuery1") false 0 "ForDuration"))
      (if (not _returnvalue_3)
        (goto _label)))))

(fn ShouldJumpDown?
  (bind _returnvalue (Transformation|GetActorLocation))
  (bind _returnvalue_2 (Transformation|GetActorForwardVector))
  (bind _charactermovement (Variables|Character|GetCharacterMovement))
  (bind _returnvalue_3 (- _returnvalue "0, 0,50.000000"))
  (bind _returnvalue_4 (* _returnvalue_2 1e+02))
  (bind _returnvalue_5 (+ _returnvalue_3 _returnvalue_4))
  (if (AI|Components|NavMovement|IsFalling _charactermovement)
    _
    (elif (> (Math|Vector|VectorLength (Variables|/Script/Engine.MovementComponent|GetVelocity _charactermovement)) 1e+01)
      (bind _returnvalue_6 (Collision|LineTraceByChannel _returnvalue_5 (- _returnvalue_5 "0, 0,100.000000") "TraceTypeQuery1" true 0 "None"))
      (if _returnvalue_6
        (return false)
        (else
          (return true)))
      (else
        _)))
  (return false))