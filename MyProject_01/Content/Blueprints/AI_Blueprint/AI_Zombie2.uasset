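; Zombie AI character that hunts players but avoids sunlight, attacking only from shade.
; Each Tick it picks the nearest visible player in front from its overlap sphere and capsule-traces toward the directional light for sun exposure.
; It then chases shaded players, wanders, or retreats to its last shade spot, using traces to jump ledges and obstacles.
; Damage retargets it to the traced hitter and ragdolls it at zero health.
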(event OnComponentBeginOverlap(Sphere)
  (params (OverlappedComponent :type Primitive%20Component%20Object%20Reference) (OtherActor :type Actor%20Object%20Reference) (OtherComp :type Primitive%20Component%20Object%20Reference) (OtherBodyIndex :type Integer) (bFromSweep :type Boolean) (SweepResult :type Hit%20Result%20Structure%20%28by%20ref%29))
  ;[1 1 1] Storing Players in array when in range
  (bind _ascharacter (Utilities|Casting|CastToCharacter OtherActor))
  (if (Pawn|IsPlayerControlled _ascharacter)
    (Utilities|Array|Add (Variables|Default|GetPlayers%20In%20Range) _ascharacter)))

(event OnComponentEndOverlap(Sphere)
  (params (OverlappedComponent :type Primitive%20Component%20Object%20Reference) (OtherActor :type Actor%20Object%20Reference) (OtherComp :type Primitive%20Component%20Object%20Reference) (OtherBodyIndex :type Integer))
  (bind _players_in_range (Variables|Default|GetPlayers%20In%20Range))
  ;[1 1 1] Storing Players in array when in range
  (bind _ascharacter (Utilities|Casting|CastToCharacter OtherActor))
  (if (Pawn|IsPlayerControlled _ascharacter)
    (if (Utilities|Array|IsValidIndex _players_in_range (Utilities|Array|FindItem _players_in_range _ascharacter))
      (Utilities|Array|RemoveItem _players_in_range _ascharacter))))

(event Custom|Move%20to%20Shade
  (bind _last_shade_location (Variables|Default|GetLast%20Shade%20Location))
  (bind (_location _rotation) (Math|Transform|BreakTransform _last_shade_location))
  (bind _returnvalue (Math|Vector|GetForwardVector _rotation))
  (bind _returnvalue_2 (* _returnvalue -1e+02))
  (bind _returnvalue_3 (+ _location _returnvalue_2))
  ;[1 1 1] Moving to shade
  (Utilities|FlowControl|DoOnce false :!label _label
    (:Completed
      (Rendering|Debug|DrawDebugSphere _returnvalue_3 1e+02 12 "(R=1.000000,G=1.000000,B=1.000000,A=1.000000)" 0.0 1e+01)
      (AI|AIMoveTo self _returnvalue_3 0 5.0 false
        (:OnSuccess
          (goto _label Reset))
        (:OnFail
          (goto _label Reset))))))

(event Custom|Go%20to%20Player
  ;[1 1 1] Going to player location
  (Utilities|FlowControl|DoOnce false :!label _label
    (:Completed
      (AI|AIMoveTo self "0, 0, 0" (Variables|Default|GetPlayer%20in%20front) (select (Math|Random|RandomBool) 1.5e+02 8e+01) false
        (:OnSuccess
          (goto _label Reset))
        (:OnFail
          (goto _label Reset))))))

(event Custom|When%20In%20sun
  (bind _player_in_front (Variables|Default|GetPlayer%20In%20front))
  ;[1 1 1] Update Whne in sunlight
  (Utilities|FlowControl|Sequence
    (:then_0
      (Utilities|IsValid (Variables|Default|GetPlayer%20In%20front)
        (:Is%20Valid
          (if (Variables|Default|GetIn%20sun)
            (bind _asplayer_character_bp (Utilities|Casting|CastToPlayerCharacterBP _player_in_front))
            (if (Variables|/Game/Blueprints/PlayerBlueprint/PlayerCharacterBP.PlayerCharacterBP_C|GetIn%20Sunlight%20? _asplayer_character_bp)
              (CallFunction|ROSSetRotation (Math|Rotator|MakeRotator 0.0 0.0 (.yaw (CallFunction|RotationtoPlayer))))
              (Utilities|FlowControl|DoOnce false :!label _label
                (:Completed
                  (Components|Movement|StopMovementImmediately (Variables|Character|GetCharacterMovement))))
              (else
                (CallFunction|GotoPlayer :!label _label_2)
                (goto _label Reset)))
            (else
              (bind _asplayer_character_bp_2 (Utilities|Casting|CastToPlayerCharacterBP _player_in_front))
              (if (not (Variables|/Game/Blueprints/PlayerBlueprint/PlayerCharacterBP.PlayerCharacterBP_C|GetIn%20Sunlight%20? _asplayer_character_bp_2))
                (goto _label_2)))))
        (:Is%20Not%20Valid
          (if (Variables|Default|GetIn%20sun)
            (CallFunction|MovetoShade)
            (else
              (CallFunction|Move))))))
    (:then_1
      (if (not (Variables|Default|GetIn%20sun))
        (Variables|Default|SetLast%20Shade%20Location (Transformation|GetActorTransform))))))

(event Custom|Move
  ;[1 1 1] Move to Random Location
  (Utilities|FlowControl|DoOnce false :!label _label
    (:Completed
      (AI|AIMoveTo self (.RandomLocation (Class|NavigationSystem|GetRandomPointinNavigableRadius (Transformation|GetActorLocation) 5e+03)) 0 5.0 false
        (:OnSuccess
          _)
        (:OnFail
          _))
      (Utilities|FlowControl|Delay 5.0)
      (goto _label Reset))))

(event Game|Damage|EventAnyDamage
  (params (Damage :type Float%20%28single-precision%29) (DamageType :type Damage%20Type%20Object%20Reference) (InstigatedBy :type Controller%20Object%20Reference) (DamageCauser :type Actor%20Object%20Reference))
  (bind _output_get (Variables|Default|SetHealth (- (Variables|Default|GetHealth) Damage)))
  (Utilities|FlowControl|Sequence
    (:then_0
      (CallFunction|ROSMontage "/Game/GameContent/Animations/WareWolfAnimations/A_hit_body_front_Montage.A_hit_body_front_Montage")
      (bind _ascharacter (Utilities|GetHitter (Transformation|GetActorLocation DamageCauser))
        (:Found
          (Variables|Default|SetPlayer%20In%20front _ascharacter)
          (CallFunction|GotoPlayer))))
    (:then_1
      (if (not (> _output_get 0.0))
        (Variables|Default|SetIs%20Dead true)
        (Physics|SetSimulatePhysics (Variables|Character|GetMesh) true)
        (Utilities|FlowControl|Delay 5.0)
        (Actor|DestroyActor)))))

(event EventTick
  (params (DeltaSeconds :type Float%20%28single-precision%29))
  (if (not (Variables|Default|GetIs%20Dead))
    (Utilities|FlowControl|Sequence
      (:then_0
        (CallFunction|LookforPlayer)
        (CallFunction|InDirectSunLight?)
        (CallFunction|WheninSun))
      (:then_1
        (Utilities|JumpDown?)
        (Utilities|JumponThings?)
        (Utilities|AttackPlayer)))))

(event EventBeginPlay
  (CallFunction|Move))

(event Custom|ROS_Montage
  (params (AnimMontage :type Anim%20Montage%20Object%20Reference))
  (Networking|SwitchHasAuthority
    (:Authority
      (Animation|PlayAnimMontage AnimMontage 1.0 "None"))))

(event Custom|ROS_Movement%20mode
  (params (NewMovementMode :type EMovementMode%20Enum :default "MOVE_None"))
  (Networking|SwitchHasAuthority
    (:Authority
      (Pawn|Components|CharacterMovement|SetMovementMode (Variables|Character|GetCharacterMovement) NewMovementMode 0))))

(event Custom|ROS_Set%20Rotation
  (params (NewRotation :type Rotator))
  (Networking|SwitchHasAuthority
    (:Authority
      (Transformation|SetActorRotation NewRotation))))

(fn ConstructionScript)

(fn GetPlayerinFront
  (bind _players_in_range (Variables|Default|GetPlayers%20In%20Range))
  (bind _players_in_front (LocalVariables|GetPlayers%20In%20front))
  (bind _distance_of_front_players (LocalVariables|GetDistance%20of%20front%20players))
  (bind _indexofminvalue (Math|Float|MinOfFloatArray _distance_of_front_players))
  (bind _output (Utilities|Array|Get(acopy) _players_in_front _indexofminvalue))
  (Utilities|IsValid (Utilities|Array|Get(acopy) _players_in_range)
    (:Is%20Valid
      (for _array_element _players_in_range
        (Development|PrintString (Utilities|String|ToString(Float) (Math|Float|Absolute(Float) (.yaw (Math|Rotator|Delta(Rotator) (Math|Rotator|FindLookatRotation (Transformation|GetActorLocation) (Transformation|GetActorLocation _array_element)) (Transformation|GetActorRotation))))) true false "(R=1.000000,G=1.000000,B=1.000000,A=1.000000)" 0.0)
        (if (< (Math|Float|Absolute(Float) (.yaw (Math|Rotator|Delta(Rotator) (Math|Rotator|FindLookatRotation (Transformation|GetActorLocation) (Transformation|GetActorLocation _array_element)) (Transformation|GetActorRotation)))) 1.1e+02)
          (Development|PrintString "In front" true false "(R=1.000000,G=0.000000,B=0.000000,A=1.000000)" 0.0)
          (Utilities|Array|Add (LocalVariables|GetPlayers%20In%20front) _array_element)
          (Utilities|Array|Add (LocalVariables|GetDistance%20of%20front%20players) (Transformation|GetDistanceTo _array_element))))
      (Utilities|IsValid _output
        (:Is%20Valid
          (return _output))
        (:Is%20Not%20Valid
          _)))
    (:Is%20Not%20Valid
      _))
  (return 0))

(fn LookforPlayer
  (bind _player_in_front (CallFunction|GetPlayerinFront))
  (Utilities|IsValid _player_in_front
    (:Is%20Valid
      (bind _outhit (Collision|LineTraceByChannel (Transformation|GetSocketLocation (Variables|Character|GetMesh) "Head") (Transformation|GetSocketLocation (Variables|/Script/Engine.Character|GetMesh _player_in_front) "Head") "TraceTypeQuery2" true 0 "ForOneFrame" true "(R=1.000000,G=0.000000,B=1.000000,A=1.000000)" "(R=1.000000,G=1.000000,B=1.000000,A=1.000000)"))
      (bind _ascharacter (Utilities|Casting|CastToCharacter (.HitActor (Collision|BreakHitResult _outhit)))
        (:then
          (Variables|Default|SetPlayer%20In%20front _ascharacter))
        (:CastFailed
          (Variables|Default|SetPlayer%20In%20front 0))))))

(fn InDirectSunLight?
  (bind _returnvalue (Transformation|GetActorLocation))
  (bind _outactors (Actor|GetAllActorsOfClass "/Script/Engine.DirectionalLight"))
  (bind (_outhit _returnvalue_2) (Collision|CapsuleTraceByChannel _returnvalue (+ _returnvalue (* (Math|Vector|GetForwardVector (Transformation|GetActorRotation (Utilities|Array|Get(acopy) _outactors))) -99999.0)) 34.0 88.0 "TraceTypeQuery2" false 0 "None" true "(R=0.000000,G=0.233631,B=1.000000,A=1.000000)" "(R=1.000000,G=1.000000,B=1.000000,A=1.000000)"))
  (if _returnvalue_2
    (Variables|Default|SetIn%20sun false)
    (else
      (Variables|Default|SetIn%20sun true))))

(fn RotationtoPlayer
  (bind _player_in_front (Variables|Default|GetPlayer%20in%20front))
  (Utilities|IsValid _player_in_front
    (:Is%20Valid
      (return (Math|Rotator|MakeRotator 0.0 0.0 (.yaw (Math|Rotator|FindLookatRotation (Transformation|GetActorLocation) (Transformation|GetActorLocation _player_in_front))))))
    (:Is%20Not%20Valid
      (return "0, 0, 0"))))